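; MyPlayerUnit is the player unit Blueprint, which creates and feeds the player's on-screen HUD.
; BeginPlay creates a HUD_BP widget, stores a reference to it and adds it to the viewport.
; Every Tick pushes the unit's state into that widget, covering health, ammo, reload, pickups, keys and the current interactable.
; Health and reload are normalized for display, and journal name and text are copied only while reading a journal terminal.
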(event EventBeginPlay
  (bind _returnvalue (UserInterface|CreateWidget "/Game/UI/HUD_BP.HUD_BP_C"))
  (bind _output_get (Variables|Default|SetHUDRefrence _returnvalue))
  (UserInterface|Viewport|AddtoViewport _output_get 0))

(event Collision|EventActorBeginOverlap
  (params (OtherActor :type Actor%20Object%20Reference)))

(event EventTick
  (params (DeltaSeconds :type Float%20%28single-precision%29))
  (bind _hudrefrence (Variables|Default|GetHUDRefrence))
  (bind _hudrefrence_2 (Variables|Default|GetHUDRefrence))
  (bind _hudrefrence_3 (Variables|Default|GetHUDRefrence))
  (bind _readingjournalterminal (Variables|Default|GetReadingJournalTerminal))
  (Variables|/Game/UI/HUD_BP.HUD_BP_C|SetActiveItem _hudrefrence (Variables|Default|GetCurrentInteractableUnit))
  (Variables|/Game/UI/HUD_BP.HUD_BP_C|SetHealthbarPercentage _hudrefrence (Math|Float|NormalizetoRange (Variables|Default|GetCurrentHealth) 0.0 (Variables|Default|GetMaxHealth)))
  (Variables|/Game/UI/HUD_BP.HUD_BP_C|SetAmmoCount _hudrefrence (Variables|Default|GetCurrentMagazineAmmo))
  (Variables|/Game/UI/HUD_BP.HUD_BP_C|SetHealthPackCount _hudrefrence (Variables|Default|GetHealthPackCount))
  (Variables|/Game/UI/HUD_BP.HUD_BP_C|SetAmmoToDisplay _hudrefrence (Variables|Default|GetAmmoStringToDisplay))
  (Variables|/Game/UI/HUD_BP.HUD_BP_C|SetHasItem _hudrefrence (Variables|Default|GetbInRangeOfItem))
  (Variables|/Game/UI/HUD_BP.HUD_BP_C|SetJournalOpen _hudrefrence_3 _readingjournalterminal)
  (if _readingjournalterminal
    (Variables|/Game/UI/HUD_BP.HUD_BP_C|SetJournalName _hudrefrence_3 (Variables|Default|GetJournalName))
    (Variables|/Game/UI/HUD_BP.HUD_BP_C|SetJournalText _hudrefrence_3 (Variables|Default|GetJournalText)))
  ;[1 1 1] Comment
  (Variables|/Game/UI/HUD_BP.HUD_BP_C|SetReloadPercentage _hudrefrence_2 (Math|Float|NormalizetoRange (Variables|Default|GetcurrentReloadTime) 0.0 (Variables|Default|GetReloadTime)))
  (Variables|/Game/UI/HUD_BP.HUD_BP_C|SetIsReloading _hudrefrence_2 (Variables|Default|GetbIsReloading))
  (Variables|/Game/UI/HUD_BP.HUD_BP_C|SetPlayersKeyAmount (Variables|Default|GetHUDRefrence) (Variables|Default|GetKeyAmount)))

(fn ConstructionScript)